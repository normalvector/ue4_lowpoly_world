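; BP_Globe is a procedural planet with a displaced terrain surface and a scaled sea sphere, rebuilt in the construction script.
; RebuildGlobeSurface reuses GlobeStaticMesh for the sea and copies its sections into the procedural SurfaceMesh with collision.
; Each terrain vertex is pushed along its normalized direction between MinHeight and MaxHeight by CalculateHeightAtPoint, a summed per-axis sine wave.
; An inward radial force setup exists in the event graph but never runs.
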(event EventBeginPlay)

(fn ConstructionScript
  (CallFunction|RebuildGlobeSurface))

(fn RebuildGlobeSurface
  (bind _globestaticmesh (Variables|Surface|GetGlobeStaticMesh))
  (bind _seaheight (Variables|Default|GetSeaHeight))
  (bind _returnvalue (* _seaheight 0.02))
  (Utilities|FlowControl|Sequence
    (:then_0
      ;[1 1 1] Use the GlobeStaticMesh for the sea
      (Components|StaticMesh|SetStaticMesh (Variables|Default|GetSeaMesh) (Variables|Surface|GetGlobeStaticMesh))
      ;[1 1 1] Use the provided SeaMaterial
      (Rendering|Material|SetMaterial (Variables|Default|GetSeaMesh) 0 (Variables|Default|GetSeaMaterial))
      ;[1 1 1] As globe mesh radius = 0.5 scale to SeaHeight x2.
      (Transformation|SetRelativeScale3D (Variables|Default|GetSeaMesh) (Math|Vector|MakeVector _returnvalue _returnvalue _returnvalue)))
    (:then_1
      ;[1 1 1] Delete all existing geometry
      (Class|ProceduralMeshComponent|ClearAllMeshSections (Variables|Default|GetSurfaceMesh)))
    (:then_2
      ;[1 1 1] Set the Globe's Material
      (Rendering|Material|SetMaterial (Variables|Default|GetSurfaceMesh) 0 (Variables|Surface|GetGlobeSurfaceMaterial)))
    (:then_3
      ;[1 1 1] Get data from static mesh
      ;;[1 1 1] Iterate over the sections of Globe Static Mesh
      (for _index (range 0 (- (Class|StaticMesh|GetNumSections _globestaticmesh) 1))
        ;;[1 1 1] Clear the transformed vertices
        (Utilities|Array|Clear (LocalVariables|GetTransformedVertices))
        ;;[1 1 1] Get the mesh data
        (bind (_vertices _triangles _normals _uvs) (Class|KismetProceduralMeshLibrary|GetSectionfromStaticMesh _globestaticmesh 0 _index))
        ;[1 1 1] Calculte TransformedVertices using the CalculateHeightAtPoint method
        (for _array_element _vertices
          (Utilities|Array|Add (LocalVariables|GetTransformedVertices) (* (Math|Vector|Normalize _array_element) (Math|Float|Lerp (Variables|Surface|GetMinHeight) (Variables|Surface|GetMaxHeight) (.Height (CallFunction|CalculateHeightatPoint _array_element))))))
        ;[1 1 1] Create a new PCM Section with transformed mesh data
        (Class|ProceduralMeshComponent|CreateMeshSectionLinearColor (Variables|Default|GetSurfaceMesh) 0 (LocalVariables|GetTransformedVertices) _triangles 0 _uvs 0 0 true)))))

(fn CalculateHeightatPoint
  (params (Position :type Vector))
  (bind _returnvalue (Math|Vector|Normalize Position))
  (bind _heightfrequency (Variables|Surface|GetHeightFrequency))
  (bind _returnvalue_2 (* _returnvalue _heightfrequency))
  (bind (_x _y _z) (Math|Vector|BreakVector _returnvalue_2))
  (return (Math|Float|Clamp(Float) (/ (+ (Math|Trig|Sin(Radians) _x) (Math|Trig|Sin(Radians) _y) (Math|Trig|Sin(Radians) _z) 3.0) 6.0)) 0.0))