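; An actor component intended to apply radial gravity to actors that carry a BP_GlobePhysicsComponent; the force itself is unfinished.
; On BeginPlay it scans every actor in the world, caches all such components in an array and prints their owners' names for debugging.
; ApplyGravitationalForce only loops over that array with an empty body and is not called here, while its static mesh AddRadialForce nodes are left disconnected.
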(event EventBeginPlay
  (CallFunction|UpdateGlobePhysicsComponentList)
  (for _array_element (Variables|Default|GetGlobePhysicsComponents)
    (Development|PrintString (Utilities|GetDisplayName (Components|GetOwner _array_element)) true true "(R=1.000000,G=0.000000,B=0.323000,A=1.000000)" 1.2e+02)))

(fn UpdateGlobePhysicsComponentList
  (Utilities|FlowControl|Sequence
    (:then_0
      ;[1 1 1] Clear out the list of components
      (Utilities|Array|Clear (Variables|Default|GetGlobePhysicsComponents)))
    (:then_1
      ;[1 1 1] Iterate over all Actors in the game world
      (bind _outactors (Actor|GetAllActorsOfClass "/Script/Engine.Actor"))
      (for _array_element _outactors
        ;[1 1 1] Find all GlobePhysicsComponents attached to this actor
        (for _array_element_2 (Actor|GetComponentsByClass _array_element "/Game/Blueprints/BP_GlobePhysicsComponent.BP_GlobePhysicsComponent_C")
          ;[1 1 1] Add them to our array
          (Utilities|Array|Add (Variables|Default|GetGlobePhysicsComponents) _array_element_2))))))

(fn ApplyGravitationalForce
  ;[1 1 1] Iterate over the GlobePhysicsComponents
  (for _array_element (Variables|Default|GetGlobePhysicsComponents)
    _))